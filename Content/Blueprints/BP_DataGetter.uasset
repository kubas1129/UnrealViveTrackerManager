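; BP_DataGetter is an actor that collects transforms from tracked VR devices of type Other and distributes them as sensor data.
; Every tick it polls their position and orientation into the DataList map keyed by device ID, firing add or update dispatchers.
; Each new device spawns a BP_Visualization, and while devices are present the map's values go to SendData.
; BeginPlay opens the WB_ControlMenu widget, and helper functions read or overwrite entries by ID.
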(event `self.ReceiveBeginPlay`
  (bind _returnvalue (`GameplayStatics.GetPlayerController` 0))
  (bind _returnvalue_2 (`|CreateWidget` "/Game/UI/WB_ControlMenu.WB_ControlMenu_C" _returnvalue self))
  (`UserWidget.AddToViewport` _returnvalue_2 0)
  (`WidgetBlueprintLibrary.SetInputMode_GameAndUIEx` _returnvalue _returnvalue_2))

(event `self.ReceiveTick`
  (params (DeltaSeconds :type "Float (single-precision)"))
  (bind _outtrackeddeviceids (`SteamVRFunctionLibrary.GetValidTrackedDeviceIds` "Other"))
  (if (> (`KismetArrayLibrary.Array_Length` _outtrackeddeviceids) 0)
    (for _array_element _outtrackeddeviceids
      (bind (_value _returnvalue) (`BlueprintMapLibrary.Map_Find` (`self.DataList`) _array_element))
      (if _returnvalue
        (bind (_outposition _outorientation) (`SteamVRFunctionLibrary.GetTrackedDevicePositionAndOrientation` _array_element))
        (bind _returnvalue_2 (`KismetMathLibrary.MakeTransform` _outposition _outorientation))
        (bind _structout (setmembers `SensorDataStruct` :`StructRef` _value :`Position` _returnvalue_2))
        (`BlueprintMapLibrary.Map_Add` (`self.DataList`) _array_element _structout)
        (`self.OnSensorUpdate` _array_element)
        (else
          (`BlueprintMapLibrary.Map_Add` (`self.DataList`) _array_element (make `SensorDataStruct` _array_element "Anchor" 0 _returnvalue_2))
          (`self.OnSensorAdd` _array_element)
          (`|SpawnActorFromClass` "/Game/Blueprints/BP_Visualization.BP_Visualization_C" (`KismetMathLibrary.MakeTransform` (0.0 0.0 0.0)) "Undefined" "OverrideRootScale" null self null))))
    (bind _values (`BlueprintMapLibrary.Map_Values` (`self.DataList`)))
    (`self.SendData` _values)))

(fn `GetSensorById`
  (params (SensorId :type Integer))
  (returns (SensorData :type "SensorDataStruct Structure"))
  (bind (_value _returnvalue) (`BlueprintMapLibrary.Map_Find` (`self.DataList`) SensorId))
  (if _returnvalue
    (return _value)
    (else
      (return))))

(fn `SetSensorDataForId`
  (params (Key :type "Integer (by ref)") (Value :type "SensorDataStruct Structure (by ref)"))
  (`BlueprintMapLibrary.Map_Add` (`self.DataList`) Key Value))

(fn `UserConstructionScript`)